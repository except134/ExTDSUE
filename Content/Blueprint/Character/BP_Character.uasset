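; Top-down character Blueprint that handles camera zoom and walk, sprint and aim input.
; Construction sets the boom's length, rotation and lag; the mouse wheel then zooms within height limits, either instantly or in looping-timer steps that block new slides until done.
; Walk, sprint and aim inputs set flags and call ChangeMovementState, whose body is not in this file.
; CameraShakeEvent plays a world camera shake at the camera's location.
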(event Input|ActionEvents|InputActionAimEvent
  (params (Key :type Key%20Structure))
  (:Pressed
    (Variables|Default|SetAimEnabled true)
    (Class|ExTDSUECharacter|ChangeMovementState :!label _label))
  (:Released
    (Variables|Default|SetAimEnabled false)
    (goto _label)))

(event Input|ActionEvents|InputActionChangeToSprint
  (params (Key :type Key%20Structure))
  (:Pressed
    (Variables|Default|SetSprintRunEnabled true)
    (Class|ExTDSUECharacter|ChangeMovementState :!label _label))
  (:Released
    (Variables|Default|SetSprintRunEnabled false)
    (goto _label)))

(event Input|ActionEvents|InputActionChangeToWalk
  (params (Key :type Key%20Structure))
  (:Pressed
    (Variables|Default|SetWalkEnabled true)
    (Class|ExTDSUECharacter|ChangeMovementState :!label _label))
  (:Released
    (Variables|Default|SetWalkEnabled false)
    (goto _label)))

(event Input|AxisEvents|InputAxisMouseWheel
  (params (AxisValue :type Float%20%28single-precision%29))
  (if (Variables|Camera|Main|GetSlideWithSmooth)
    (CallFunction|CameraSlideSmooth AxisValue)
    (else
      (CallFunction|CameraSlide AxisValue))))

(event Input|KeyboardEvents|LeftAlt
  (params (Key :type Key%20Structure)))

(fn ConstructionScript
  (bind _cameraboom (Variables|Default|GetCameraBoom))
  (Variables|/Script/Engine.SpringArmComponent|SetTargetArmLength _cameraboom (Variables|Camera|Main|GetHeightCameraMin))
  (Transformation|SetRelativeRotation _cameraboom (Variables|Camera|Main|GetRotatorCamera) false false)
  (Variables|/Script/Engine.SpringArmComponent|SetbEnableCameraLag _cameraboom (Variables|Camera|Main|GetFlow))
  (Variables|/Script/Engine.SpringArmComponent|SetCameraLagSpeed _cameraboom (Variables|Camera|Main|GetCoeffSmooth)))

(fn CameraShakeEvent
  (Camera|PlayWorldCameraShake "/Game/Blueprint/Game/BP_ShakeCamera.BP_ShakeCamera_C" (Transformation|GetWorldLocation (Variables|Default|GetTopDownCameraComponent)) 0.0 3e+01)
  (return))

(fn CameraSlide
  (params (InputPin :type Float%20%28single-precision%29))
  (bind _heightcamerachangedistance (Variables|Camera|Slide|GetHeightCameraChangeDistance))
  (bind _cameraboom (Variables|Default|GetCameraBoom))
  (if (!= InputPin 0.0)
    (if (< InputPin 0.0)
      (if (>= (Variables|Camera|Main|GetHeightCameraMax) (+ (Variables|/Script/Engine.SpringArmComponent|GetTargetArmLength _cameraboom) _heightcamerachangedistance))
        (Variables|/Script/Engine.SpringArmComponent|SetTargetArmLength _cameraboom (+ (Variables|/Script/Engine.SpringArmComponent|GetTargetArmLength _cameraboom) _heightcamerachangedistance)))
      (elif (<= (Variables|Camera|Main|GetHeightCameraMin) (- (Variables|/Script/Engine.SpringArmComponent|GetTargetArmLength _cameraboom) _heightcamerachangedistance))
        (Variables|/Script/Engine.SpringArmComponent|SetTargetArmLength _cameraboom (- (Variables|/Script/Engine.SpringArmComponent|GetTargetArmLength _cameraboom) _heightcamerachangedistance))))))

(fn CameraSlideSmooth
  (params (InputPin :type Float%20%28single-precision%29))
  (bind _cameraboom (Variables|Default|GetCameraBoom))
  (bind _heightcamerachangedistance (Variables|Camera|Slide|GetHeightCameraChangeDistance))
  (bind _targetarmlength (Variables|/Script/Engine.SpringArmComponent|GetTargetArmLength _cameraboom))
  (if (Variables|Camera|Slide|GetSlideDone)
    (if (!= InputPin 0.0)
      (if (< InputPin 0.0)
        (if (>= (Variables|Camera|Main|GetHeightCameraMax) (+ _targetarmlength _heightcamerachangedistance))
          (Variables|Camera|Slide|SetSlideUp true)
          (Variables|Camera|Slide|SetSlideDone false :!label _label)
          (bind _returnvalue (Utilities|Time|SetTimerbyFunctionName 0 "CameraSlideSmoothTick" (Variables|Camera|Slide|GetTimerStep) true))
          (Variables|Camera|Slide|SetSlideTimer _returnvalue))
        (elif (<= (Variables|Camera|Main|GetHeightCameraMin) (- _targetarmlength _heightcamerachangedistance))
          (Variables|Camera|Slide|SetSlideUp false)
          (goto _label))))))

(fn CameraSlideSmoothTick
  (bind _heightcamerachangeslidestepdistance (Variables|Camera|Slide|GetHeightCameraChangeSlideStepDistance))
  (bind _cameraboom (Variables|Default|GetCameraBoom))
  (bind _output_get (Variables|Camera|Slide|SetCurrentSlideDistance (+ (Variables|Camera|Slide|GetCurrentSlideDistance) _heightcamerachangeslidestepdistance)))
  (Variables|/Script/Engine.SpringArmComponent|SetTargetArmLength _cameraboom (select (Variables|Camera|Slide|GetSlideUp) (+ (Variables|/Script/Engine.SpringArmComponent|GetTargetArmLength _cameraboom) _heightcamerachangeslidestepdistance) (- (Variables|/Script/Engine.SpringArmComponent|GetTargetArmLength _cameraboom) _heightcamerachangeslidestepdistance)))
  (if (>= _output_get (Variables|Camera|Slide|GetHeightCameraChangeDistance))
    (Variables|Camera|Slide|SetCurrentSlideDistance 0.0)
    (Variables|Camera|Slide|SetSlideDone true)
    (Utilities|Time|ClearandInvalidateTimerbyHandle (Variables|Camera|Slide|GetSlideTimer))))